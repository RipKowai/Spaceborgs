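; Health pickup actor that heals the first-person player character on overlap.
; A looping timeline bobs and spins the pickup mesh, storing the last rotation as the start of the next cycle.
; Box overlap adds a fixed amount of health, capped at MaxHealth, then destroys the actor; a player at full health leaves it in place.
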(event `self.ReceiveBeginPlay`
  ;[1 0.9815 0.6995] Set values at begin play
  (set `self.CurrentTransform` (`KismetMathLibrary.Conv_VectorToTransform` (`SceneComponent.K2_GetComponentLocation` (`self.PickUp`))))
  (`self.MovePickup`))

(event `MovePickup`
  (bind _currenttransform_location (`KismetMathLibrary.BreakTransform` (`self.CurrentTransform`)))
  (bind _currenttransform_location_2 (`KismetMathLibrary.BreakTransform` (`self.CurrentTransform`)))
  ;[0.8658 0.6317 1] Rotation and moving pickup
  (bind (_direction _location _rotation) (`Timeline|Timeline` :!via `PlayFromStart`)
    (:`Update`
      (bind _returnvalue_location (`KismetMathLibrary.BreakTransform` (`KismetMathLibrary.TLerp` (`KismetMathLibrary.MakeTransform` _currenttransform_location_2) (`KismetMathLibrary.MakeTransform` (+ _currenttransform_location (0.0 0.0 50.0)) (struct :`Pitch` 200.0 :`Roll` 200.0)) _location)))
      (bind (_returnvalue_location_2 _returnvalue_rotation) (`KismetMathLibrary.BreakTransform` (`KismetMathLibrary.TLerp` (`KismetMathLibrary.MakeTransform` (0.0 0.0 0.0) (`self.newRot`)) (`KismetMathLibrary.MakeTransform` (0.0 0.0 0.0) (struct :`Pitch` 1000.0 :`Yaw` 1000.0 :`Roll` 1000.0)) _rotation)))
      (`SceneComponent.K2_SetWorldTransform` (`self.PickUp`) (`KismetMathLibrary.MakeTransform` _returnvalue_location _returnvalue_rotation (0.6 0.6 0.6)) false false))
    (:`Finished`
      (set `self.newRot` _returnvalue_rotation)
      (`self.MovePickup`))))

(event `self.Box.OnComponentBeginOverlap`
  (params (OverlappedComponent :type "PrimitiveComponent Object Reference") (OtherActor :type "Actor Object Reference") (OtherComp :type "PrimitiveComponent Object Reference") (OtherBodyIndex :type Integer) (bFromSweep :type Boolean) (SweepResult :type "HitResult Structure (by ref)"))
  (bind _firstpersonref (`self.FirstPersonRef`))
  (bind _maxhealth (`SpaceborgsCharacter.MaxHealth` (`self.FirstPersonRef`)))
  (bind _returnvalue (+ (`SpaceborgsCharacter.Health` (`self.FirstPersonRef`)) 30.0))
  ;[0.6244 0.9801 1] Health Logic. If added health is greater than max, set health to maxHealth.
  (bind _asbp_first_person_character (cast `/Game/FirstPerson/Blueprints/BP_FirstPersonCharacter` OtherActor))
  (set `self.FirstPersonRef` _asbp_first_person_character)
  (if (< (`SpaceborgsCharacter.Health` _firstpersonref) (`SpaceborgsCharacter.MaxHealth` _firstpersonref))
    (if (> _returnvalue _maxhealth)
      (set `SpaceborgsCharacter.Health` _maxhealth (`self.FirstPersonRef`))
      (`self.K2_DestroyActor`)
      (else
        (set `SpaceborgsCharacter.Health` _returnvalue (`self.FirstPersonRef`))
        (`self.K2_DestroyActor`)))))

(fn `UserConstructionScript`)