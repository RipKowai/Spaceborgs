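; BP_Door is a door that raises when a player character carrying a key overlaps its box trigger.
; The overlap calls OpenDoor and clears the player's key, or prints a missing-key message.
; OpenDoor runs only while KeyOpenable is false, using a timeline to lerp the door mesh upward.
; The timeline's first update also tells EnemySpawnLocation to spawn enemies, guarded by IsTriggered to fire once.
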(event `Open Door`
  (if (not (`self.KeyOpenable`))
    (bind (_direction _doorfloat) (`Timeline|Timeline`)
      (:`Update`
        (`SceneComponent.K2_SetRelativeLocation` (`self.modular_door`) (`KismetMathLibrary.MakeVector` 0.0 0.0 (`KismetMathLibrary.Lerp` 0.0 300.0 _doorfloat)) false false)
        (if (not (`self.IsTriggered`))
          (`SpawnLocation.SpawnEnemies` (`self.EnemySpawnLocation`))
          (set `self.IsTriggered` true))))))

(event `self.Box.OnComponentBeginOverlap`
  (params (OverlappedComponent :type "PrimitiveComponent Object Reference") (OtherActor :type "Actor Object Reference") (OtherComp :type "PrimitiveComponent Object Reference") (OtherBodyIndex :type Integer) (bFromSweep :type Boolean) (SweepResult :type "HitResult Structure (by ref)"))
  (bind _asbp_first_person_character (cast `/Game/FirstPerson/Blueprints/BP_FirstPersonCharacter` OtherActor))
  (if (`SpaceborgsCharacter.HasKey` _asbp_first_person_character)
    (`self.Open Door`)
    (set `SpaceborgsCharacter.HasKey` false _asbp_first_person_character)
    (else
      (`KismetSystemLibrary.PrintString` "You dont have a key!!! \nFind DA KEY!!!"))))

(fn `UserConstructionScript`)