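; Enemy AI character that spots and melees the first-person player, takes damage and ragdolls on death.
; Pawn sensing sets a blackboard seen-player flag, cleared by a retriggerable two-second delay; death sets another.
; AttackPlayer sphere-traces forward, plays a montage, then damages players in a debug-drawn sphere overlap on its notify.
; Tick updates the camera-facing health bar against a hardcoded maximum; damage triggers a blood splash.
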(event `self.ReceiveTick`
  (params (DeltaSeconds :type "Float (single-precision)"))
  (bind _health_bar_widget (`self.Health Bar Widget`))
  (if (not (`self.HasDied`))
    (bind _asw_enemy_health_bar (cast `/Game/Evert_Andersson/W_EnemyHealthBar` (`WidgetComponent.GetWidget` (`self.Health Bar Widget`))))
    (`ProgressBar.SetPercent` (`/Game/Evert_Andersson/W_EnemyHealthBar.HealthBar` _asw_enemy_health_bar) (/ (`self.Health`) 20.0))
    (`SceneComponent.K2_SetWorldRotation` _health_bar_widget (`KismetMathLibrary.FindLookAtRotation` (`SceneComponent.K2_GetComponentLocation` _health_bar_widget) (`SceneComponent.K2_GetComponentLocation` (`PlayerCameraManager.TransformComponent` (`GameplayStatics.GetPlayerCameraManager` 0)))) false false)))

(event `self.PawnSensing.OnSeePawn`
  (params (Pawn :type "Pawn Object Reference"))
  (cast `/Game/FirstPerson/Blueprints/BP_FirstPersonCharacter` Pawn)
  (`BlackboardComponent.SetValueAsBool` (`AIBlueprintHelperLibrary.GetBlackboard` (`AIBlueprintHelperLibrary.GetAIController` self)) "HasSeenPlayer?" true)
  (`KismetSystemLibrary.RetriggerableDelay` 2.0)
  (`BlackboardComponent.SetValueAsBool` (`AIBlueprintHelperLibrary.GetBlackboard` (`AIBlueprintHelperLibrary.GetAIController` self)) "HasSeenPlayer?" false))

(event `AttackPlayer`
  (bind _returnvalue (`self.K2_GetActorLocation`))
  (bind _returnvalue_2 (`SceneComponent.K2_GetComponentLocation` (`self.Sphere`)))
  (if (not (`self.HasDied`))
    (bind (_outhit _returnvalue_3) (`KismetSystemLibrary.SphereTraceSingleForObjects` :`Start` _returnvalue :`End` (+ _returnvalue (* (`KismetMathLibrary.GetForwardVector` (`self.K2_GetActorRotation`)) 250.0)) :`Radius` 120.0 :`ObjectTypes` (`|MakeArray` "ObjectTypeQuery3" :!type "EObjectTypeQuery Enum") :`DrawDebugType` "ForDuration"))
    (if _returnvalue_3
      (cast `/Game/FirstPerson/Blueprints/BP_FirstPersonCharacter` (`.HitActor` (`GameplayStatics.BreakHitResult` _outhit)))
      (`|PlayMontage` (`self.Mesh`) "/Game/LiamAnderberg/Enemy_AI/Animation/Attack.Attack"
        (:`then`
          (`GameplayStatics.PlaySound2D` "/Engine/EditorSounds/Notifications/CompileSuccess.CompileSuccess" 0.5 1.0 0.0 null null))
        (:`OnNotifyBegin`
          (bind _outactors (`KismetSystemLibrary.SphereOverlapActors` _returnvalue_2 (`self.Attack Radius`) (`|MakeArray` "ObjectTypeQuery3" :!type "EObjectTypeQuery Enum") "/Game/FirstPerson/Blueprints/BP_FirstPersonCharacter.BP_FirstPersonCharacter_C" (`|MakeArray` self :!type "Actor Object Reference")))
          (`KismetSystemLibrary.DrawDebugSphere` _returnvalue_2 (`self.Attack Radius`) 12 (struct :`R` 1.0 :`B` 0.050657 :`A` 1.0) (`self.Attack Duration`))
          (for _array_element _outactors
            (bind _asbp_first_person_character (cast `/Game/FirstPerson/Blueprints/BP_FirstPersonCharacter` _array_element))
            (`SpaceborgsCharacter.TakePlayerDamage` _asbp_first_person_character (`self.Attack Base Damage`))))))))

(event `Take Damage`
  (params (Damage :type "Float (double-precision)"))
  (bind _health (`self.Health`))
  (`ActorComponent.Activate` (`self.BloodSplash`) true)
  (set `self.Health` (- _health Damage))
  (if (<= _health 0.0)
    (`self.Die`)))

(event `Die`
  (set `self.HasDied` true)
  (`PrimitiveComponent.SetSimulatePhysics` (`self.Mesh`) true)
  (`BlackboardComponent.SetValueAsBool` (`AIBlueprintHelperLibrary.GetBlackboard` (`AIBlueprintHelperLibrary.GetAIController` self)) "HasDied" true)
  (`PrimitiveComponent.SetCollisionEnabled` (`self.CapsuleComponent`) "NoCollision")
  (`SceneComponent.SetHiddenInGame` (`self.Health Bar Widget`) true false))

(fn `UserConstructionScript`)